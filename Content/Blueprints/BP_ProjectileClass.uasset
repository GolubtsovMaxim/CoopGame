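; A timed explosive projectile Actor that detonates shortly after spawning, with no impact handling in its graph.
; BeginPlay waits on a short fixed delay, then calls Explode, which spawns an explosion particle and applies full radial damage within DamageRadius, credited to its instigator controller.
; It then destroys itself and draws a debug sphere showing the blast radius.
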(event `self.ReceiveBeginPlay`
  (`KismetSystemLibrary.Delay` 0.8)
  (`self.Explode`))

(event `Explode`
  (bind _returnvalue (`self.K2_GetActorLocation`))
  (`GameplayStatics.SpawnEmitterAtLocation` "/Game/WeaponEffects/Explosion/P_Explosion.P_Explosion" _returnvalue)
  (`GameplayStatics.ApplyRadialDamage` :`BaseDamage` 100.0 :`Origin` _returnvalue :`DamageRadius` (`self.DamageRadius`) :`DamageCauser` self :`InstigatedByController` (`self.GetInstigatorController`) :`bDoFullDamage` true)
  (`self.K2_DestroyActor`)
  (`KismetSystemLibrary.DrawDebugSphere` _returnvalue (`self.DamageRadius`) 12 (struct :`R` 0.734375 :`G` 0.051446 :`B` 0.102633 :`A` 1.0) 1.0 2.0))

(fn `UserConstructionScript`)